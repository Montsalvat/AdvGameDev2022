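; Player controller that translates movement, jump and mouse-look input into actions on the controlled character.
; BeginPlay casts the controlled pawn to Character and caches it for the movement and jump events.
; Movement axes push the character along the camera manager's forward and right vectors, so motion follows the view direction.
; Mouse axes feed controller pitch and yaw directly, while the jump action starts and stops the character's jump.
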(event EventBeginPlay
  (bind _ascharacter (Utilities|Casting|CastToCharacter (Pawn|GetControlledPawn)))
  (Variables|Default|SetCharacterRef _ascharacter))

(event Input|ActionEvents|InputActionJump
  (params (Key :type Key%20Structure :default "None"))
  (bind _characterref (Variables|Default|GetCharacterRef))
  ;[1 1 1] Jumping
  (:Pressed
    (Character|Jump _characterref))
  (:Released
    (Character|StopJumping _characterref)))

(event Input|AxisEvents|InputAxisMoveForward/Backwards
  (params (AxisValue :type Float%20%28single-precision%29))
  ;[1 1 1] Player Movement
  (Pawn|Input|AddMovementInput (Variables|Default|GetCharacterRef) (Transformation|GetActorForwardVector (Variables|Default|GetPlayerCameraManager)) AxisValue false))

(event Input|AxisEvents|InputAxisMoveRight/Left
  (params (AxisValue :type Float%20%28single-precision%29))
  ;[1 1 1] Player Movement
  (Pawn|Input|AddMovementInput (Variables|Default|GetCharacterRef) (Transformation|GetActorRightVector (Variables|Default|GetPlayerCameraManager)) AxisValue false))

(event Input|AxisEvents|InputAxisMousePitch
  (params (AxisValue :type Float%20%28single-precision%29))
  ;[1 1 1] Camera Player Rotation
  (Class|PlayerController|AddPitchInput AxisValue))

(event Input|AxisEvents|InputAxisMouseYaw
  (params (AxisValue :type Float%20%28single-precision%29))
  ;[1 1 1] Camera Player Rotation
  (Class|PlayerController|AddYawInput AxisValue))

(fn ConstructionScript)